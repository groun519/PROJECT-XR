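; BP_GameQuit is an actor that hosts the WBP_GameQuit game-quit menu through a widget component.
; On BeginPlay it binds the widget's close request to CloseWidget.
; Closing destroys the actor, clears the QuitNPC's clicked flag, picks it a random rise animation index and removes the IMC_Menu input mapping context from the first player.
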(event Custom|Close%20Widget
  (bind _quit_npc (Variables|Default|GetQuit%20NPC))
  (Actor|DestroyActor)
  (Variables|/Game/WorkSpace/UI/UI_Test/Blueprint/BP_NPC/BP_BaseNPC.BP_BaseNPC_C|SetIs%20Clicked? _quit_npc false)
  (Variables|/Game/WorkSpace/UI/UI_Test/Blueprint/BP_NPC/BP_BaseNPC.BP_BaseNPC_C|SetRise%20Anim%20Index _quit_npc (Math|Random|RandomIntegerinRange 0 2))
  (Input|RemoveMappingContext (PlayerController|LocalPlayerSubsystems|GetEnhancedInputLocalPlayerSubsystem (Game|GetPlayerController 0)) "/Game/VRTemplate/Input/IMC_Menu.IMC_Menu" "(bIgnoreAllPressedKeysUntilRelease=True,bForceImmediately=False,bNotifyUserSettings=False)"))

(event EventBeginPlay
  (|CallParentFunction)
  (bind _aswbp_game_quit (Utilities|Casting|CastToWBP_GameQuit (UserInterface|GetUserWidgetObject (Variables|Default|GetWidget))))
  (EventDispatchers|BindEventtoRequestClose _aswbp_game_quit (delegate Custom|Close%20Widget)))

(fn ConstructionScript)