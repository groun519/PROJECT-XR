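; Base NPC Blueprint that reacts to hover and click with a highlight, a text label and random animation picks.
; BeginPlay creates dynamic body and head materials, whose GlowSwitch toggles with label visibility on hover.
; Hover start picks a HoverAnimIndex; the first click picks a DeathAnimIndex and blocks further hover starts.
; TextRenderSetting attaches the label to the Head socket; yaw-to-camera logic is left unwired.
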(event Custom|Clicked
  (if (not (Variables|Default|GetIs%20Clicked?))
    (Variables|Default|SetIs%20Clicked? true)
    (Variables|Default|SetDeath%20Anim%20Index (Math|Random|RandomIntegerinRange 0 2))))

(event Custom|Hover%20Start
  (if (not (Variables|Default|GetIs%20Clicked?))
    (if (not (Variables|Default|GetIs%20Hovered?))
      (Variables|Default|SetIs%20Hovered? true)
      (Utilities|FlowControl|Sequence
        (:then_0
          (Rendering|Material|SetScalarParameterValue (Variables|Default|GetHead%20DM) "GlowSwitch" 1.0 :!class /Script/Engine.MaterialInstanceDynamic)
          (Rendering|Material|SetScalarParameterValue (Variables|Default|GetBody%20DM) "GlowSwitch" 1.0 :!class /Script/Engine.MaterialInstanceDynamic))
        (:then_1
          (Rendering|SetVisibility (Variables|Default|GetTextRender) true false))
        (:then_2
          (Variables|Default|SetHover%20Anim%20Index (Math|Random|RandomIntegerinRange 0 3)))))))

(event Custom|Hover%20End
  (if (Variables|Default|GetIs%20Hovered?)
    (Variables|Default|SetIs%20Hovered? false)
    (Utilities|FlowControl|Sequence
      (:then_0
        (Rendering|Material|SetScalarParameterValue (Variables|Default|GetHead%20DM) "GlowSwitch" 0.0 :!class /Script/Engine.MaterialInstanceDynamic)
        (Rendering|Material|SetScalarParameterValue (Variables|Default|GetBody%20DM) "GlowSwitch" 0.0 :!class /Script/Engine.MaterialInstanceDynamic))
      (:then_1
        (Rendering|SetVisibility (Variables|Default|GetTextRender) false false)))))

(event EventBeginPlay
  (CallFunction|MakeDynamicMats (Variables|Character|GetMesh) (Variables|Character|GetMesh)))

(event EventTick
  (params (DeltaSeconds :type Float%20%28single-precision%29)))

(fn ConstructionScript)

(fn MakeDynamicMats
  (params (Body%20Mesh%20Input :type Skeletal%20Mesh%20Component%20Object%20Reference) (Head%20Mesh%20Input :type Skeletal%20Mesh%20Component%20Object%20Reference))
  (Utilities|FlowControl|Sequence
    (:then_0
      (bind _returnvalue (Rendering|Material|CreateDynamicMaterialInstance Body%20Mesh%20Input 0 0 "None" :!class /Script/Engine.PrimitiveComponent))
      (bind _output_get (Variables|Default|SetBody%20DM _returnvalue))
      (Rendering|Material|SetMaterial Body%20Mesh%20Input 0 _output_get))
    (:then_1
      (bind _returnvalue_2 (Rendering|Material|CreateDynamicMaterialInstance Head%20Mesh%20Input 1 0 "None" :!class /Script/Engine.PrimitiveComponent))
      (bind _output_get_2 (Variables|Default|SetHead%20DM _returnvalue_2))
      (Rendering|Material|SetMaterial Head%20Mesh%20Input 1 _output_get_2))))

(fn TextRenderSetting
  (params (Text :type Text))
  (Transformation|AttachComponentToComponent (Variables|Default|GetTextRender) (Variables|Character|GetMesh) "Head" "SnapToTarget" "SnapToTarget" "KeepRelative" true)
  (Transformation|SetRelativeLocationAndRotation (Variables|Default|GetTextRender) "50.000000,0.000000,0.000000" "0.000000,90.000000,-90.000000" false false)
  (Rendering|Components|TextRender|SetText (Variables|Default|GetTextRender) Text))