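; BP_MonsterBase is a monster base that spawns Target actors on its body and takes damage by rank.
; Each living Tick picks head, body or leg height and line-traces toward it from a randomly offset horizontal start, retrying after short delays on failure.
; A self-hit spawns a linked Target at the impact point.
; CauseDamage lowers HP; at zero, Die ragdolls the mesh and Tick destroys the actor after a delay.
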(event Custom|Add%20Target
  (params (BodyType :type BodyType%20Enum :default "BodyType_MAX"))
  (bind _returnvalue (Transformation|GetActorLocation))
  (Variables|Default|SetEndVector _returnvalue)
  (Variables|Default|SetStartVector _returnvalue)
  (switch Utilities|FlowControl|Switch|SwitchonBodyType BodyType
    (:NewEnumerator0
      (Variables|Default|SetEndVector (+ (Variables|Default|GetEndVector) "0.000000,0.000000,75.000000")))
    (:NewEnumerator1
      (Variables|Default|SetEndVector (+ (Variables|Default|GetEndVector) "0.000000,0.000000,10.000000")))
    (:NewEnumerator2
      (Variables|Default|SetEndVector (+ (Variables|Default|GetEndVector) "0.000000,0.000000,-30.000000"))))
  (bind _output_get (Variables|Default|SetRandX (Math|Random|RandomFloatinRange -1e+03 1e+03)))
  (bind _output_get_2 (Variables|Default|SetRandY (Math|Random|RandomFloatinRange -1e+03 1e+03)))
  (bind _output_get_3 (Variables|Default|SetRandZ (Math|Random|RandomFloatinRange 0.0 0.0)))
  (bind _output_get_4 (Variables|Default|SetStartVector (+ (Variables|Default|GetStartVector) (Math|Vector|MakeVector _output_get _output_get_2 _output_get_3))))
  (bind _output_get_5 (Variables|Default|SetTrace%20Channel "TraceTypeQuery4"))
  (bind (_outhit _returnvalue_2) (Collision|LineTraceByChannel _output_get_4 (Variables|Default|GetEndVector) _output_get_5 false 0 "ForDuration" false))
  (if _returnvalue_2
    (if (Actor|ActorHasTag "Target")
      (Utilities|FlowControl|Delay 0.01 :!label _label)
      (CallFunction|ReFindImpactPoint)
      (elif (== (.HitActor (Collision|BreakHitResult _outhit)) self)
        (bind _returnvalue_3 (Game|SpawnActorfromClass "/Game/Target.Target_C" (Math|Transform|MakeTransform (.ImpactPoint (Collision|BreakHitResult _outhit)) (Math|Rotator|FindLookatRotation (Variables|Default|GetStartVector) (Variables|Default|GetEndVector)) "0.200000,0.200000,0.200000") "Undefined" "MultiplyWithRoot" 0 0))
        (Variables|/Game/Target.Target_C|SetTargetMonster _returnvalue_3 self)
        (else
          (goto _label))))
    (else
      (goto _label))))

(event Custom|ReFindImpactPoint
  (bind _output_get (Variables|Default|SetRandX (Math|Random|RandomFloatinRange -1e+03 1e+03)))
  (bind _output_get_2 (Variables|Default|SetRandY (Math|Random|RandomFloatinRange -1e+03 1e+03)))
  (bind _output_get_3 (Variables|Default|SetRandZ (Math|Random|RandomFloatinRange 0.0 0.0)))
  (bind _output_get_4 (Variables|Default|SetStartVector (+ (Variables|Default|GetStartVector) (Math|Vector|MakeVector _output_get _output_get_2 _output_get_3))))
  (bind _output_get_5 (Variables|Default|SetTrace%20Channel "TraceTypeQuery4"))
  (bind (_outhit _returnvalue) (Collision|LineTraceByChannel _output_get_4 (Variables|Default|GetEndVector) _output_get_5 false 0 "ForDuration" false))
  (if _returnvalue
    (if (Actor|ActorHasTag "Target")
      (Utilities|FlowControl|Delay 0.01 :!label _label)
      (CallFunction|ReFindImpactPoint)
      (elif (== (.HitActor (Collision|BreakHitResult _outhit)) self)
        (bind _returnvalue_2 (Game|SpawnActorfromClass "/Game/Target.Target_C" (Math|Transform|MakeTransform (.ImpactPoint (Collision|BreakHitResult _outhit)) (Math|Rotator|FindLookatRotation (Variables|Default|GetStartVector) (Variables|Default|GetEndVector)) "0.200000,0.200000,0.200000") "Undefined" "MultiplyWithRoot" 0 0))
        (Variables|/Game/Target.Target_C|SetTargetMonster _returnvalue_2 self)
        (else
          (goto _label))))
    (else
      (goto _label))))

(event EventBeginPlay)

(event Collision|EventActorBeginOverlap
  (params (OtherActor :type Actor%20Object%20Reference)))

(event EventTick
  (params (DeltaSeconds :type Float%20%28single-precision%29))
  (if (Variables|Default|GetbIsDied)
    (Utilities|FlowControl|Delay 1.0)
    (Actor|DestroyActor)
    (else
      (CallFunction|AddTarget (.OutItem (Utilities|Array|Random (Utilities|Array|MakeArray "NewEnumerator0" "NewEnumerator1" "NewEnumerator2")))))))

(fn ConstructionScript)

(fn CauseDamage
  (params (Rank :type TargetRank%20Enum :default "NewEnumerator0"))
  (switch Utilities|FlowControl|Switch|SwitchonTargetRank Rank
    (:NewEnumerator0
      (LocalVariables|SetDamage 1))
    (:NewEnumerator1
      (LocalVariables|SetDamage 2))
    (:NewEnumerator2
      (LocalVariables|SetDamage 3))
    (:NewEnumerator3
      (LocalVariables|SetDamage 4)))
  (bind _output_get (Variables|Default|SetHP (- (Variables|Default|GetHP) (LocalVariables|GetDamage))))
  (Development|PrintString (Utilities|String|Append (Utilities|GetDisplayName self) "Remaining HP : " (Utilities|String|ToString(Integer) _output_get)))
  (if (<= _output_get 0)
    (Development|PrintString (Utilities|String|Append (Utilities|GetDisplayName self) "Is Died!") true true "(R=1.000000,G=0.011039,B=0.000000,A=1.000000)")
    (CallFunction|Die)))

(fn Die
  (bind _mesh (Variables|Character|GetMesh))
  (Collision|SetCollisionProfileName _mesh "Ragdoll" true :!class /Script/Engine.PrimitiveComponent)
  (Physics|SetSimulatePhysics _mesh true)
  (Variables|Default|SetbIsDied true))