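; BP_Projectile is a damage-dealing projectile actor that can hurt both monsters and the VR player.
; InitData stores the damage amount passed in by the caller.
; When its StaticMesh begins an overlap, it checks Monster or Player tags, casts to BP_MonsterBase or VRPawn, and calls CauseDamage.
; It destroys itself on a fixed timer after BeginPlay, not on impact.
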(event OnComponentBeginOverlap(StaticMesh)
  (params (OverlappedComponent :type Primitive%20Component%20Object%20Reference) (OtherActor :type Actor%20Object%20Reference) (OtherComp :type Primitive%20Component%20Object%20Reference) (OtherBodyIndex :type Integer) (bFromSweep :type Boolean) (SweepResult :type Hit%20Result%20Structure%20%28by%20ref%29))
  (if (Actor|ActorHasTag OtherActor "Monster")
    (bind _asbp_monster_base (Utilities|Casting|CastToBP_MonsterBase OtherActor))
    (Default|CauseDamage _asbp_monster_base (Variables|Default|GetDamage))
    (elif (Actor|ActorHasTag OtherActor "Player")
      (bind _asvrpawn (Utilities|Casting|CastToVRPawn OtherActor))
      (Default|CauseDamage _asvrpawn (Variables|Default|GetDamage)))))

(event Custom|InitData
  (params (Damage :type Float%20%28double-precision%29))
  (Variables|Default|SetDamage Damage))

(event EventBeginPlay
  (Utilities|FlowControl|Delay 1e+01)
  (Actor|DestroyActor))

(event Collision|EventActorBeginOverlap
  (params (OtherActor :type Actor%20Object%20Reference)))

(fn ConstructionScript)