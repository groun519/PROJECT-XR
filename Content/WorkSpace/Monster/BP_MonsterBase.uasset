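; Base monster Blueprint that wanders around its spawn point and chases and attacks pawns it sees within MaxDistance.
; Tick moves a spawned TargetActor to random line-traced points, drives AIMoveTo, and drops combat when out of range.
; PawnSensing switches the target and headgear color; reaching it plays a random montage that briefly enables weapon overlaps.
; CauseDamage lowers Health and can trigger Die, which ragdolls the mesh before delayed destruction.
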(event OnSeePawn(PawnSensing)
  (params (Pawn :type Pawn%20Object%20Reference))
  ;[1 1 1] 시야에 Pawn이 발견되었을 때
  ;[1 1 1] 전투 범위 내부인가?
  (if (not (Variables|MoveTarget|GetbIsFarToOrigin))
    ;[1 1 1] 타겟을 대상으로 변경
    (Variables|Combat|SetisCombat true)
    (CallFunction|SetTarget Pawn)
    (CallFunction|SetHeadGearColor "(R=1.000000,G=0.000000,B=0.014251,A=1.000000)")))

(event Custom|AttackAction
  (bind _attackmontages (Variables|Default|GetAttackMontages))
  ;[1 1 1] 공격액션
  (if (not (Variables|MoveTarget|GetbIsAttacking))
    (Variables|MoveTarget|SetbIsAttacking true)
    ;[1 1 1] 몽타주 실행
    (bind _notifyname (Animation|Montage|PlayMontage (Variables|Character|GetMesh) (.AttackMontage (Utilities|Struct|BreakAttackMontageInfo (Utilities|Array|Get(acopy) _attackmontages (Math|Random|RandomIntegerinRange 0 (Utilities|Array|Length _attackmontages))))))
      (:OnCompleted
        (Utilities|FlowControl|Delay 0.2 :!label _label)
        ;[1 1 1] 끝나면 다시 움직임
        (Variables|MoveTarget|SetbIsMoving false)
        (Variables|MoveTarget|SetbIsAttacking false))
      (:OnBlendOut
        (goto _label))
      (:OnInterrupted
        (goto _label))
      (:OnNotifyBegin
        ;[1 1 1] Attack 노티파이를 만나면
        (if (== _notifyname "Attack")
          ;[1 1 1] 콜리전 0.2초간 활성화
          (Variables|/Script/Engine.PrimitiveComponent|SetbGenerateOverlapEvents (Variables|Default|GetWeaponMesh) true)
          (Utilities|FlowControl|Delay 0.2)
          (Variables|/Script/Engine.PrimitiveComponent|SetbGenerateOverlapEvents (Variables|Default|GetWeaponMesh) false))))))

(event Custom|Turn
  (bind _returnvalue (Transformation|GetActorRotation))
  (bind _returnvalue_2 (Transformation|GetActorLocation))
  (bind _target (Variables|Combat|GetTarget))
  (bind _returnvalue_3 (Transformation|GetActorLocation _target))
  (bind _returnvalue_4 (Math|Rotator|FindLookatRotation _returnvalue_2 _returnvalue_3))
  ;[1 1 1] 액터 회전
  (Transformation|SetActorRotation (Math|Rotator|MakeRotator 0.0 0.0 (Math|Interpolation|FInterpTo (.yaw _returnvalue) (.yaw _returnvalue_4) (Utilities|Time|GetWorldDeltaSeconds) 5.0)))
  (if (< (Math|Float|Absolute(Float) (- (.yaw _returnvalue) (.yaw _returnvalue_4))) 1.0)
    (Variables|Default|SetbIsTurn false)
    (Utilities|Time|ClearandInvalidateTimerbyHandle (Variables|Default|GetHandle))
    (Development|PrintString "Hello")
    (else
      (Variables|Default|SetbIsTurn true))))

(event Custom|TurnMonster
  ;[1 1 1] 액터 회전
  (Variables|Default|SetbIsTurn true)
  (bind _returnvalue (Utilities|Time|SetTimerbyEvent (delegate Custom|Turn) 0.01 true))
  (Variables|Default|SetHandle _returnvalue))

(event EventBeginPlay
  ;[1 1 1] 게임 시작 시 1회
  ;[1 1 1] 몬스터 위치에 OriginActor(전투 종료시 되돌아갈 지점) 생성 후 변수로 저장
  (bind _returnvalue (Game|SpawnActorfromClass "/Game/WorkSpace/Monster/OriginActor.OriginActor_C" (Transformation|GetActorTransform) "Undefined" "MultiplyWithRoot" 0 0))
  (Variables|MoveTarget|SetOriginActor _returnvalue)
  ;[0.7042 0.2889 1] 범위 디버그
  (Rendering|Debug|DrawDebugSphere (Transformation|GetActorLocation _returnvalue) (Variables|MoveTarget|GetMaxDistance) 12 "(R=1.000000,G=1.000000,B=1.000000,A=1.000000)" 1e+03)
  ;[1 1 1] 타겟 액터(전투 대상이 없을 때 따라다닐 액터) 생성 및 변수로 저장
  (bind _returnvalue_2 (Game|SpawnActorfromClass "/Game/WorkSpace/Monster/TargetActor.TargetActor_C" (Transformation|GetActorTransform (Variables|MoveTarget|GetOriginActor)) "Undefined" "MultiplyWithRoot" 0 0))
  (bind _output_get (Variables|MoveTarget|SetTargetActor _returnvalue_2))
  (CallFunction|SetTarget _output_get)
  (CallFunction|SetHeadGearColor "(R=0.027762,G=0.000000,B=1.000000,A=1.000000)"))

(event EventTick
  (params (DeltaSeconds :type Float%20%28single-precision%29))
  (bind _returnvalue (Utilities|Time|GetGameTimeinSeconds))
  (bind _maxdistance (Variables|MoveTarget|GetMaxDistance))
  (bind _originactor (Variables|MoveTarget|GetOriginActor))
  (bind _targetactor (Variables|MoveTarget|GetTargetActor))
  (bind _returnvalue_2 (Transformation|GetActorLocation _originactor))
  (bind _returnvalue_3 (* _returnvalue _maxdistance))
  (bind (_x _y _z) (Math|Vector|BreakVector _returnvalue_2))
  ;[1 1 1] 매 1초 반복루프
  (Utilities|FlowControl|Sequence
    (:then_0
      ;[1 1 1] OriginActor에서 MaxDistance만큼 떨어져서 전투범위 밖으로 이동했는가?
      (bind _output_get (Variables|MoveTarget|SetbIsFarToOrigin (>= (Math|Vector|Distance(Vector) (Transformation|GetActorLocation (Variables|MoveTarget|GetOriginActor)) (Transformation|GetActorLocation)) (Variables|MoveTarget|GetMaxDistance))))
      (if _output_get
        ;[1 1 1] 전투상태 해제 -> 타겟을 OriginActor로 변경
        (Variables|Combat|SetisCombat false)
        (CallFunction|SetTarget)
        (CallFunction|SetHeadGearColor "(R=0.027762,G=0.000000,B=1.000000,A=1.000000)")))
    (:then_1
      (if (not (Variables|Combat|GetisCombat))
        (Utilities|FlowControl|Sequence
          (:then_0
            ;[1 1 1] 움직이는 중인가?
            (if (not (Variables|MoveTarget|GetbIsMoving))
              ;[0.7042 0.2889 1] 목적지 디버그
              (Rendering|Debug|DrawDebugSphere (Transformation|GetActorLocation (Variables|MoveTarget|GetTargetActor)) 1e+02 12 "(R=1.000000,G=0.000000,B=0.000000,A=1.000000)" 5.0 3.0)
              ;[1 1 1] 원점 기준 사용할 랜덤한 거리 연산
              (Utilities|IsValid (Variables|MoveTarget|GetTargetActor)
                (:Is%20Valid
                  (Variables|MoveTarget|SetRandomDistance (Math|Random|RandomFloatinRange (/ (Variables|MoveTarget|GetMaxDistance) 4.0) (Variables|MoveTarget|GetMaxDistance)))
                  ;[1 1 1] 원형 범위 벡터 연산
                  (bind _output_get_2 (Variables|MoveTarget|SetRandomDest (Math|Vector|MakeVector (+ (* (Math|Trig|Cos(Degrees) _returnvalue_3) (Variables|MoveTarget|GetRandomDistance)) _x) (+ (* (Math|Trig|Sin(Degrees) _returnvalue_3) (Variables|MoveTarget|GetRandomDistance)) _y) _z)))
                  ;[1 1 1] 랜덤 벡터 위치 z벡터 + 1000에서 레이 발사 -> 충돌지점을 목표지점으로 지정.
                  (bind _outhit (Collision|LineTraceByChannel (+ _output_get_2 "0.000000,0.000000,1000.000000") (+ _output_get_2 "0.000000,0.000000,-1000.000000") "TraceTypeQuery1" false 0 "ForDuration"))
                  ;[1 1 1] 목표지점으로 Target Actor 이동 후 Target으로 지정
                  (Transformation|SetActorLocation _targetactor (.ImpactPoint (Collision|BreakHitResult _outhit)) false false)
                  (CallFunction|SetTarget _targetactor))))))))
    (:then_2
      ;[1 1 1] 움직이는 중인가?
      (if (not (Variables|MoveTarget|GetbIsMoving))
        ;[1 1 1] Target에게 이동
        (Variables|MoveTarget|SetbIsMoving true)
        (AI|AIMoveTo self "0, 0, 0" (Variables|Combat|GetTarget) 5.0 true
          (:OnSuccess
            ;[1 1 1] 전투중인가?
            (if (Variables|Combat|GetisCombat)
              ;[1 1 1] Yes : 공격
              (CallFunction|AttackAction)
              (else
                ;[1 1 1] No : 다시 움직임
                (Variables|MoveTarget|SetbIsMoving false)))))))
    (:then_3
      (if (Variables|Combat|GetbIsDead)
        (Utilities|FlowControl|Delay 1.0)
        (Actor|DestroyActor)))))

(fn ConstructionScript)

(fn CauseDamage
  (params (Damage :type Float%20%28double-precision%29))
  (bind _output_get (Variables|Default|SetHealth (- (Variables|Default|GetHealth) Damage)))
  (Development|PrintString (Utilities|String|Append (Utilities|GetDisplayName self) "Remaining HP : " (Utilities|String|ToString(Float) _output_get)))
  (if (<= 0.0 _output_get)
    (Development|PrintString (Utilities|String|Append (Utilities|GetDisplayName self) "Is Died!") true true "(R=1.000000,G=0.011039,B=0.000000,A=1.000000)")
    (CallFunction|Die)))

(fn Die
  (bind _mesh (Variables|Character|GetMesh))
  (Collision|SetCollisionProfileName _mesh "Ragdoll" true :!class /Script/Engine.PrimitiveComponent)
  (Physics|SetSimulatePhysics _mesh true)
  (Variables|Combat|SetbIsDead true))

(fn MosterFindPlayer
  (bind _originactor (Variables|MoveTarget|GetOriginActor))
  (bind _returnvalue (Transformation|GetDistanceTo _originactor 0))
  (if (not (Variables|MoveTarget|GetbIsFarToOrigin))
    (Development|PrintString (Utilities|String|ToString(Float) _returnvalue) true true "(R=1.000000,G=0.269233,B=0.000000,A=1.000000)")
    (if (< _returnvalue (/ (Variables|MoveTarget|GetMaxDistance) 2.0))
      (return))))

(fn SetTarget
  (params (NewTarget :type Actor%20Object%20Reference))
  (Variables|Combat|SetTarget NewTarget)
  (Variables|MoveTarget|SetbIsMoving false))

(fn SetHeadGearColor
  (params (Color :type Linear%20Color%20Structure))
  (bind _headgearmesh (Variables|Default|GetHeadGearMesh))
  (Development|PrintString (Utilities|String|ToString(Integer) Color))
  (bind _returnvalue (Rendering|Material|CreateDynamicMaterialInstance _headgearmesh 0 (Rendering|Material|GetMaterial _headgearmesh 0) "Color" :!class /Script/Engine.PrimitiveComponent))
  (Rendering|Material|SetVectorParameterValue _returnvalue "Color" Color :!class /Script/Engine.MaterialInstanceDynamic))