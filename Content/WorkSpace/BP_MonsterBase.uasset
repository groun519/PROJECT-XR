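; Base monster that roams around its spawn point, chases seen pawns and carries hittable weak-point targets.
; Tick periodically moves a target actor around a spawned origin actor to wander, and returns the monster home past MaxDistance.
; AddTarget line-traces from random offsets toward head, body or leg, retrying until it can place a Target on the monster's surface.
; CauseDamage subtracts HP by rank, and Die ragdolls the mesh.
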(event OnSeePawn(PawnSensing)
  (params (Pawn :type Pawn%20Object%20Reference))
  (if (not (Variables|Default|GetisFarToMaxDistance))
    (AI|AIMoveTo self (Transformation|GetActorLocation Pawn) 0 5.0 true
      (:then
        (Variables|Default|SetisCombat true)))))

(event Custom|Add%20Target
  (params (BodyType :type BodyType%20Enum :default "BodyType_MAX"))
  (bind _returnvalue (Transformation|GetActorLocation))
  (Variables|Default|SetEndVector _returnvalue)
  (Variables|Default|SetStartVector _returnvalue)
  (switch Utilities|FlowControl|Switch|SwitchonBodyType BodyType
    (:NewEnumerator0
      (Variables|Default|SetEndVector (+ (Variables|Default|GetEndVector) "0.000000,0.000000,75.000000")))
    (:NewEnumerator1
      (Variables|Default|SetEndVector (+ (Variables|Default|GetEndVector) "0.000000,0.000000,10.000000")))
    (:NewEnumerator2
      (Variables|Default|SetEndVector (+ (Variables|Default|GetEndVector) "0.000000,0.000000,-30.000000"))))
  (bind _output_get (Variables|Default|SetRandX (Math|Random|RandomFloatinRange -1e+03 1e+03)))
  (bind _output_get_2 (Variables|Default|SetRandY (Math|Random|RandomFloatinRange -1e+03 1e+03)))
  (bind _output_get_3 (Variables|Default|SetRandZ (Math|Random|RandomFloatinRange 0.0 0.0)))
  (bind _output_get_4 (Variables|Default|SetStartVector (+ (Variables|Default|GetStartVector) (Math|Vector|MakeVector _output_get _output_get_2 _output_get_3))))
  (bind _output_get_5 (Variables|Default|SetTrace%20Channel "TraceTypeQuery4"))
  (bind (_outhit _returnvalue_2) (Collision|LineTraceByChannel _output_get_4 (Variables|Default|GetEndVector) _output_get_5 false 0 "ForDuration" false))
  (if _returnvalue_2
    (if (Actor|ActorHasTag (.HitActor (Collision|BreakHitResult _outhit)) "Target")
      (Utilities|FlowControl|Delay 0.01 :!label _label)
      (CallFunction|ReFindImpactPoint)
      (elif (== (.HitActor (Collision|BreakHitResult _outhit)) self)
        (bind _returnvalue_3 (Game|SpawnActorfromClass "/Game/WorkSpace/Target.Target_C" (Math|Transform|MakeTransform (.ImpactPoint (Collision|BreakHitResult _outhit)) (Math|Rotator|FindLookatRotation (Variables|Default|GetStartVector) (Variables|Default|GetEndVector)) "0.200000,0.200000,0.200000") "Undefined" "MultiplyWithRoot" 0 0))
        (Variables|/Game/WorkSpace/Target.Target_C|SetTargetMonster _returnvalue_3 self)
        (else
          (goto _label))))
    (else
      (goto _label))))

(event Custom|ReFindImpactPoint
  (bind _output_get (Variables|Default|SetRandX (Math|Random|RandomFloatinRange -1e+03 1e+03)))
  (bind _output_get_2 (Variables|Default|SetRandY (Math|Random|RandomFloatinRange -1e+03 1e+03)))
  (bind _output_get_3 (Variables|Default|SetRandZ (Math|Random|RandomFloatinRange 0.0 0.0)))
  (bind _output_get_4 (Variables|Default|SetStartVector (+ (Variables|Default|GetStartVector) (Math|Vector|MakeVector _output_get _output_get_2 _output_get_3))))
  (bind _output_get_5 (Variables|Default|SetTrace%20Channel "TraceTypeQuery4"))
  (bind (_outhit _returnvalue) (Collision|LineTraceByChannel _output_get_4 (Variables|Default|GetEndVector) _output_get_5 false 0 "ForDuration" false))
  (if _returnvalue
    (if (Actor|ActorHasTag (.HitActor (Collision|BreakHitResult _outhit)) "Target")
      (Utilities|FlowControl|Delay 0.01 :!label _label)
      (CallFunction|ReFindImpactPoint)
      (elif (== (.HitActor (Collision|BreakHitResult _outhit)) self)
        (bind _returnvalue_2 (Game|SpawnActorfromClass "/Game/WorkSpace/Target.Target_C" (Math|Transform|MakeTransform (.ImpactPoint (Collision|BreakHitResult _outhit)) (Math|Rotator|FindLookatRotation (Variables|Default|GetStartVector) (Variables|Default|GetEndVector)) "0.200000,0.200000,0.200000") "Undefined" "MultiplyWithRoot" 0 0))
        (Variables|/Game/WorkSpace/Target.Target_C|SetTargetMonster _returnvalue_2 self)
        (else
          (goto _label))))
    (else
      (goto _label))))

(event EventBeginPlay
  (bind _returnvalue (Game|SpawnActorfromClass "/Game/WorkSpace/OriginActor.OriginActor_C" (Transformation|GetActorTransform) "Undefined" "MultiplyWithRoot" 0 0))
  (Variables|Default|SetOriginActor _returnvalue)
  (Rendering|Debug|DrawDebugSphere (Transformation|GetActorLocation _returnvalue) (Variables|Default|GetMaxDistance) 12 "(R=1.000000,G=1.000000,B=1.000000,A=1.000000)" 1e+03)
  (bind _returnvalue_2 (Game|SpawnActorfromClass "/Game/WorkSpace/TargetActor.TargetActor_C" (Math|Conversions|ToTransform(Vector) (Math|Vector|MakeVector (+ (.X (Math|Vector|BreakVector (Transformation|GetActorLocation (Variables|Default|GetOriginActor)))) 5e+02) (.Y (Math|Vector|BreakVector (Transformation|GetActorLocation (Variables|Default|GetOriginActor)))) (.Z (Math|Vector|BreakVector (Transformation|GetActorLocation (Variables|Default|GetOriginActor)))))) "Undefined" "MultiplyWithRoot" 0 0))
  (Variables|Default|SetTargetActor _returnvalue_2))

(event Collision|EventActorBeginOverlap
  (params (OtherActor :type Actor%20Object%20Reference)))

(event EventTick
  (params (DeltaSeconds :type Float%20%28single-precision%29))
  (bind _returnvalue (Utilities|Time|GetGameTimeinSeconds))
  (bind _originactor (Variables|Default|GetOriginActor))
  (bind _returnvalue_2 (Transformation|GetActorLocation _originactor))
  (bind _returnvalue_3 (* _returnvalue 1e+03))
  (bind (_x _y _z) (Math|Vector|BreakVector _returnvalue_2))
  (Utilities|FlowControl|Sequence
    (:then_1
      (bind _output_get (Variables|Default|SetisFarToMaxDistance (>= (Math|Vector|Distance(Vector) (Transformation|GetActorLocation (Variables|Default|GetOriginActor)) (Transformation|GetActorLocation)) (Variables|Default|GetMaxDistance))))
      (if _output_get
        (AI|AIMoveTo self (Transformation|GetActorLocation) (Variables|Default|GetOriginActor) 5.0 true
          (:then
            (Variables|Default|SetisCombat false)))))
    (:then_2
      (if (not (Variables|Default|GetisCombat))
        (if (== (Math|Float|Round (Math|Float|%(Float) (Utilities|Time|GetGameTimeinSeconds) 3.0)) 0)
          (Rendering|Debug|DrawDebugSphere (Transformation|GetActorLocation (Variables|Default|GetTargetActor)) 1e+02 12 "(R=1.000000,G=0.000000,B=0.000000,A=1.000000)" 5.0 3.0)
          (Development|PrintString "move")
          (if (Utilities|IsValid (Variables|Default|GetTargetActor))
            (Variables|Default|SetRadiusRandom (Math|Random|RandomFloatinRange 5e+02 1e+03))
            (Transformation|SetActorLocation (Variables|Default|GetTargetActor) (Math|Vector|MakeVector (+ (* (Math|Trig|Cos(Degrees) _returnvalue_3) (Variables|Default|GetRadiusRandom)) _x) (+ (* (Math|Trig|Sin(Degrees) _returnvalue_3) (Variables|Default|GetRadiusRandom)) _y) _z) false false)
            (Development|PrintString (Utilities|String|ToString(Vector) (Math|Vector|MakeVector (+ (* (Math|Trig|Cos(Degrees) _returnvalue_3) (Variables|Default|GetRadiusRandom)) _x) (+ (* (Math|Trig|Sin(Degrees) _returnvalue_3) (Variables|Default|GetRadiusRandom)) _y) _z)))
            (AI|AIMoveTo self (Transformation|GetActorLocation) (Variables|Default|GetTargetActor) 5.0 true)))))))

(fn ConstructionScript)

(fn CauseDamage
  (params (Rank :type TargetRank%20Enum :default "NewEnumerator0"))
  (switch Utilities|FlowControl|Switch|SwitchonTargetRank Rank
    (:NewEnumerator0
      (LocalVariables|SetDamage 1))
    (:NewEnumerator1
      (LocalVariables|SetDamage 2))
    (:NewEnumerator2
      (LocalVariables|SetDamage 3))
    (:NewEnumerator3
      (LocalVariables|SetDamage 4)))
  (bind _output_get (Variables|Default|SetHP (- (Variables|Default|GetHP) (LocalVariables|GetDamage))))
  (Development|PrintString (Utilities|String|Append (Utilities|GetDisplayName self) "Remaining HP : " (Utilities|String|ToString(Integer) _output_get)))
  (if (<= _output_get 0)
    (Development|PrintString (Utilities|String|Append (Utilities|GetDisplayName self) "Is Died!") true true "(R=1.000000,G=0.011039,B=0.000000,A=1.000000)")
    (CallFunction|Die)))

(fn Die
  (bind _mesh (Variables|Character|GetMesh))
  (Collision|SetCollisionProfileName _mesh "Ragdoll" true :!class /Script/Engine.PrimitiveComponent)
  (Physics|SetSimulatePhysics _mesh true)
  (Variables|Default|SetbIsDied true))

(fn MosterFindPlayer
  (bind _originactor (Variables|Default|GetOriginActor))
  (bind _returnvalue (Transformation|GetDistanceTo _originactor 0))
  (if (not (Variables|Default|GetisFarToMaxDistance))
    (Development|PrintString (Utilities|String|ToString(Float) _returnvalue) true true "(R=1.000000,G=0.269233,B=0.000000,A=1.000000)")
    (if (< _returnvalue (/ (Variables|Default|GetRange) 2.0))
      (return))))