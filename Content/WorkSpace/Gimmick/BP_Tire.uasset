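; BP_Tire is a physics tire hazard that knocks the player character away on contact.
; On BeginPlay the mesh simulates physics and gets an impulse along negative Y, then after seven seconds the actor spawns a new BP_Tire at its transform and destroys itself, repeating the cycle.
; Hits on bp_ThirdPersonCharacter_SF launch it away from the actor's location with an added +Y and upward boost, overriding its velocity.
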(event OnComponentHit(TireMesh)
  (params (HitComponent :type Primitive%20Component%20Object%20Reference) (OtherActor :type Actor%20Object%20Reference) (OtherComp :type Primitive%20Component%20Object%20Reference) (NormalImpulse :type Vector :default "0, 0, 0") (Hit :type Hit%20Result%20Structure%20%28by%20ref%29))
  (bind _asbp_third_person_character_sf (Utilities|Casting|CastTobp_ThirdPersonCharacter_SF OtherActor))
  (Character|LaunchCharacter _asbp_third_person_character_sf (+ (* (Math|Vector|Normalize (- (Transformation|GetActorLocation _asbp_third_person_character_sf) (Transformation|GetActorLocation))) (Math|Conversions|ToVector(Float) 1e+04)) "0.000000,3000.000000,3000.000000") true true))

(event EventBeginPlay
  (Physics|SetSimulatePhysics (Variables|Default|GetTireMesh) true)
  (Physics|AddImpulse (Variables|Default|GetTireMesh) "0.000000,-1000.000000,0.000000" "None" true)
  (Utilities|FlowControl|Delay 7.0)
  (Game|SpawnActorfromClass "BP_Tire_C" (Transformation|GetActorTransform) "Undefined" "MultiplyWithRoot" 0 0)
  (Actor|DestroyActor))

(event Collision|EventActorBeginOverlap
  (params (OtherActor :type Actor%20Object%20Reference)))

(event EventTick
  (params (DeltaSeconds :type Float%20%28single-precision%29)))

(fn ConstructionScript)