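; Grabbable cable actor that plugs into socket point actors on overlap.
; On overlapping a BP_CableSocketPoint, it attaches the cable's end to that socket's box collision and turns off overlap events on its sphere.
; Every tick it sets the plug's world rotation using the last cable particle's location as the X-axis vector.
; The grab event is present but empty.
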(event OnGrabbed(GrabComponent))

(event EventBeginPlay)

(event EventTick
  (params (DeltaSeconds :type Float%20%28single-precision%29))
  (bind _cable (Variables|Default|GetCable))
  (bind _locations (Class|CableComponent|GetCableParticleLocations _cable))
  (Transformation|SetWorldRotation (Variables|Default|GetPlug) (Math|Conversions|RotationFromXVector (Utilities|Array|Get(acopy) _locations (Utilities|Array|LastIndex _locations))) false false))

(event Collision|EventActorBeginOverlap
  (params (OtherActor :type Actor%20Object%20Reference))
  (bind _asbp_cable_socket_point (Utilities|Casting|CastToBP_CableSocketPoint OtherActor))
  (Class|CableComponent|SetAttachEndtoComponent (Variables|Default|GetCable) (Variables|/Game/WorkSpace/Gimmick/BP_CableSocketPoint.BP_CableSocketPoint_C|GetBoxCollision _asbp_cable_socket_point) "None")
  (Variables|/Script/Engine.PrimitiveComponent|SetbGenerateOverlapEvents (Variables|Default|GetSphere) false))

(fn ConstructionScript)